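; BP_newPlatform is a moving platform that travels between a start and an end position on demand.
; The StartMove event plays a timeline whose alpha lerps the relative location of NPlatHandle from StartPosition to EndPosition.
; StartBack reverses the same timeline to send it back.
; The construction script places the handle at StartPosition.
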(event `StartMove`
  (bind (_direction _alpha) (`Timeline|Timeline_0` :!label _label)
    (:`Update`
      (`SceneComponent.K2_SetRelativeLocation` (`self.nPlatHandle`) (`KismetMathLibrary.VLerp` (`self.StartPosition`) (`self.EndPosition`) _alpha) false false))))

(event `StartBack`
  (goto _label :!via `Reverse`))

(fn `UserConstructionScript`
  (`SceneComponent.K2_SetRelativeLocation` (`self.nPlatHandle`) (`self.StartPosition`) false false))