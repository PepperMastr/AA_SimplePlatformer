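; Moving platform that travels back and forth between StartPosition and EndPosition once StartPlatform is called.
; A timeline's alpha lerps PlatformHandle's relative location without sweep, and the construction script places it at StartPosition.
; At each end, a short random delay feeds a FlipFlop that alternates reversing and playing the timeline.
; StopPlatform halts the timeline but does not cancel a pending delay.
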(event `StartPlatform`
  ;[1 1 1] Platform Movement
  (bind (_direction _alpha) (`Timeline|Timeline_0` :!label _label)
    (:`Update`
      (`SceneComponent.K2_SetRelativeLocation` (`self.PlatformHandle`) (`KismetMathLibrary.VLerp` (`self.StartPosition`) (`self.EndPosition`) _alpha) false false))
    (:`Finished`
      (`KismetSystemLibrary.Delay` (`KismetMathLibrary.RandomFloatInRange` 0.5 2.0))
      (`/Engine/EditorBlueprintResources/StandardMacros.FlipFlop`
        (:`A`
          (goto _label :!via `Reverse`))
        (:`B`
          (goto _label))))))

(event `StopPlatform`
  ;[1 1 1] Platform Movement
  (goto _label :!via `Stop`))

(fn `UserConstructionScript`
  (`SceneComponent.K2_SetRelativeLocation` (`self.PlatformHandle`) (`self.StartPosition`) false false))