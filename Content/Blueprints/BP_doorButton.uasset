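; BP_doorButton is a button that toggles a linked Platform on and off.
; Its Activated_Door event plays a hit sound at the button mesh, then a FlipFlop alternates between starting the platform with a green material and stopping it with a red one.
; Despite the door naming, the nodes that open or close MyDoor and set MyLight's intensity are disconnected and never run.
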(event `Activated_Door`
  (bind _buttonmesh (`self.ButtonMesh`))
  (bind _platform (`self.Platform`))
  ;[1 1 1] Button Activated
  (`GameplayStatics.PlaySoundAtLocation` "/Game/Audio/Misc_Hits_046.Misc_Hits_046" (`SceneComponent.K2_GetComponentLocation` (`self.ButtonMesh`)) (struct) 1.0 1.0 0.0 null null null)
  (`/Engine/EditorBlueprintResources/StandardMacros.FlipFlop`
    (:`A`
      (`PrimitiveComponent.SetMaterial` _buttonmesh 0 "/Game/Materials/M_green.M_Green")
      (`/Game/Blueprints/BP_Platform02.StartPlatform` _platform))
    (:`B`
      (`PrimitiveComponent.SetMaterial` _buttonmesh 0 "/Game/Materials/M_red.M_Red")
      (`/Game/Blueprints/BP_Platform02.StopPlatform` _platform))))

(fn `UserConstructionScript`)